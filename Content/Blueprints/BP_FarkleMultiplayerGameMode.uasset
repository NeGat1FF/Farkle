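; Game mode for two-player multiplayer Farkle, played through two BP_PlayerBoardPawn actors already in the level.
; PostLogin gives each joining player the first uncontrolled board pawn.
; Five seconds after BeginPlay, it takes the first two pawns found, spawns their dice and starts the first player's turn.
; Turns alternate through each pawn's OnEndTurn event, which starts the other player's turn.
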(event `self.ReceiveBeginPlay`
  (bind _firstplayer (`self.FirstPlayer`))
  (bind _secondplayer (`self.SecondPlayer`))
  (`KismetSystemLibrary.Delay` 5.0)
  (bind _outactors (`GameplayStatics.GetAllActorsOfClass` "/Game/Blueprints/Actors/BP_PlayerBoardPawn.BP_PlayerBoardPawn_C"))
  (set `self.FirstPlayer` (`|GetArrayItem` _outactors))
  (set `self.SecondPlayer` (`|GetArrayItem` _outactors 1))
  (`BaseBoardPawn.SpawnDices` _firstplayer 0)
  (`BaseBoardPawn.SpawnDices` _secondplayer 1)
  (add `BaseBoardPawn.OnEndTurn` _firstplayer (delegate `OnFirstPlayerEndTurn`))
  (add `BaseBoardPawn.OnEndTurn` _secondplayer (delegate `OnSecondPlayerEndTurn`))
  (`BaseBoardPawn.StartTurn` _firstplayer)
  (`BaseBoardPawn.EndTurn` _secondplayer))

(event `OnFirstPlayerEndTurn`
  (`BaseBoardPawn.StartTurn` (`self.SecondPlayer`)))

(event `OnSecondPlayerEndTurn`
  (`BaseBoardPawn.StartTurn` (`self.FirstPlayer`)))

(event `self.K2_PostLogin`
  (params (NewPlayer :type "PlayerController Object Reference"))
  (bind _outactors (`GameplayStatics.GetAllActorsOfClass` "/Game/Blueprints/Actors/BP_PlayerBoardPawn.BP_PlayerBoardPawn_C"))
  (for _array_element _outactors
    (if (not (`Pawn.IsControlled` _array_element))
      (`Controller.Possess` NewPlayer _array_element)
      (break))))

(fn `UserConstructionScript`)