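; Player board pawn for a Farkle dice game that handles the player's roll and pass input and the camera movement between turns.
; On BeginPlay it adds the Farkle Enhanced Input mapping context, whose Roll and Pass actions call RollDice and PassDice.
; A timeline plays forward when OnEndTurn fires and in reverse on StartTurn, easing the camera's relative location halfway toward the track value each update.
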(event `self.ReceiveBeginPlay`
  (add `self.OnEndTurn` (delegate `OnEndTurn_Event`))
  (`parent.ReceiveBeginPlay`)
  (bind _asplayer_controller (cast `PlayerController` (`self.GetController`)))
  (message `EnhancedInputSubsystemInterface.AddMappingContext` (pcsubsystem `EnhancedInputLocalPlayerSubsystem` _asplayer_controller) "/Game/Input/FarkleInputMappingContext.FarkleInputMappingContext" 0 (struct)))

(event `OnEndTurn_Event`
  (bind _camera (`self.Camera`))
  (bind (_direction _newtrack_0) (`Timeline|Timeline` :!via `PlayFromStart` :!label _label)
    (:`Update`
      (`SceneComponent.K2_SetRelativeLocation` _camera (`KismetMathLibrary.VLerp` _newtrack_0 (`SceneComponent.RelativeLocation` _camera) 0.5) false false))))

(event `self.StartTurn`
  (goto _label :!via `ReverseFromEnd`))

(event `EnhancedInput|/Game/Input/Actions/IA_Roll`
  (params (ActionValue :type Boolean) (ElapsedSeconds :type "Float (double-precision)") (TriggeredSeconds :type "Float (double-precision)") (InputAction :type "InputAction Object Reference" :default "/Game/Input/Actions/IA_Roll.IA_Roll"))
  (:`Started`
    (`self.RollDice`)))

(event `EnhancedInput|/Game/Input/Actions/IA_Pass`
  (params (ActionValue :type Boolean) (ElapsedSeconds :type "Float (double-precision)") (TriggeredSeconds :type "Float (double-precision)") (InputAction :type "InputAction Object Reference" :default "/Game/Input/Actions/IA_Pass.IA_Pass"))
  (:`Started`
    (`self.PassDice`)))

(fn `UserConstructionScript`
  (`parent.UserConstructionScript`))