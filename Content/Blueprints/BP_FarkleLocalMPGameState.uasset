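; Game state for local two-player Farkle that alternates turns between the first two player states in PlayerArray.
; On BeginPlay it caches both players and the first player's view target, ends the second player's turn before binding its end-turn event, then starts the first player's turn.
; Each end-turn event starts the other player's turn and blends the first player controller's view to the second player's controller or back to the saved target.
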(event `self.ReceiveBeginPlay`
  (bind _playerarray (`self.PlayerArray`))
  (bind _asfarkle_player_state (cast `FarklePlayerState` (`|GetArrayItem` _playerarray)))
  (bind _output_get (set `self.FirstPlayer` _asfarkle_player_state))
  (add `FarklePlayerState.OnPlayerEndTurn` _output_get (delegate `FirstPlayerEndTurn`))
  (set `self.FirstPlayerViewTarget` (`Controller.GetViewTarget` (`PlayerState.GetPlayerController` _output_get)))
  (bind _asfarkle_player_state_2 (cast `FarklePlayerState` (`|GetArrayItem` _playerarray 1)))
  (bind _output_get_2 (set `self.SecondPlayer` _asfarkle_player_state_2))
  (`FarklePlayerState.EndTurn` _output_get_2)
  (add `FarklePlayerState.OnPlayerEndTurn` _output_get_2 (delegate `SecondPlayerEndTurn`))
  (`FarklePlayerState.StartTurn` _output_get))

(event `FirstPlayerEndTurn`
  (bind _secondplayer (`self.SecondPlayer`))
  (`FarklePlayerState.StartTurn` _secondplayer)
  (`PlayerController.SetViewTargetWithBlend` (`PlayerState.GetPlayerController` (`self.FirstPlayer`)) (`PlayerState.GetPlayerController` _secondplayer) 2.0 "VTBlend_Linear" 0.0 false))

(event `SecondPlayerEndTurn`
  (bind _firstplayer (`self.FirstPlayer`))
  (`FarklePlayerState.StartTurn` _firstplayer)
  (`PlayerController.SetViewTargetWithBlend` (`PlayerState.GetPlayerController` _firstplayer) (`self.FirstPlayerViewTarget`) 2.0 "VTBlend_Linear" 0.0 false))

(fn `UserConstructionScript`)