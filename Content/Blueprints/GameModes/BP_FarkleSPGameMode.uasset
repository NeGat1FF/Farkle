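; Game mode for single-player Farkle that asks for a target score at the start and shows the result at the end.
; On BeginPlay it pauses the game and shows a prompt widget, setting the target score and unpausing when Play or Enter submits a numeric value.
; EndGame displays a game-over widget with a red lose or green win message, depending on whether the winner is AI.
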(event `self.ReceiveBeginPlay`
  (`KismetSystemLibrary.Delay` 0.1)
  (bind _returnvalue (`|CreateWidget` "/Game/Blueprints/Widgets/WB_SingleplayerPrompt.WB_SingleplayerPrompt_C"))
  (`GameplayStatics.SetGamePaused` true)
  (`UserWidget.AddToViewport` _returnvalue 0)
  (add `Button.OnClicked` (`/Game/Blueprints/Widgets/WB_SingleplayerPrompt.PlayButton` _returnvalue) (delegate `OnClicked_Event`))
  (add `EditableTextBox.OnTextCommitted` (`/Game/Blueprints/Widgets/WB_SingleplayerPrompt.FarkleScore` _returnvalue) (delegate `OnTextCommitted_Event`)))

(event `OnClicked_Event`
  (bind _returnvalue (`KismetTextLibrary.Conv_TextToString` (`EditableTextBox.Text` (`/Game/Blueprints/Widgets/WB_SingleplayerPrompt.FarkleScore` (stale `self.ReceiveBeginPlay` _returnvalue)))))
  (if (`KismetStringLibrary.IsNumeric` _returnvalue) :!label _label
    (`self.SetTargetScore` (`KismetStringLibrary.Conv_StringToInt` _returnvalue))
    (`GameplayStatics.SetGamePaused` false)))

(event `OnTextCommitted_Event`
  (params (Text :type "Text (by ref)") (CommitMethod :type "ETextCommit Enum" :default "Default"))
  (switch `ETextCommit` CommitMethod
    (:`OnEnter`
      (goto _label))))

(event `self.EndGame`
  (params (winner :type "BaseBoardPawn Object Reference") (loser :type "BaseBoardPawn Object Reference"))
  (bind _returnvalue (`|CreateWidget` "/Game/Blueprints/Widgets/WB_GameOver.WB_GameOver_C"))
  (if (`BaseBoardPawn.bIsAI` winner)
    (bind _image_0 (`/Game/Blueprints/Widgets/WB_GameOver.Image_0` _returnvalue))
    (set `Image.ColorAndOpacity` (struct :`R` 1.0 :`A` 1.0) _image_0)
    (bind _textblock (`/Game/Blueprints/Widgets/WB_GameOver.TextBlock` _returnvalue))
    (set `TextBlock.Text` "YOU LOSE" _textblock)
    (else
      (set `Image.ColorAndOpacity` (struct :`G` 1.0 :`A` 1.0) _image_0)
      (set `TextBlock.Text` "YOU WON" _textblock)))
  (`UserWidget.AddToViewport` _returnvalue 0))

(fn `UserConstructionScript`)