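; Game mode for two-player Farkle that handles match setup, game end, restart and logout.
; BeginPlay takes an optional target score from the level's options string.
; EndGame gives both player controllers a result widget, identifying the winner by a "FirstPlayer" substring in its display name.
; RestartGame removes those widgets, zeroes both players' scores and ends SecondPlayer's turn, while logout opens the main menu level.
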(event `self.ReceiveBeginPlay`
  (bind _optionsstring (`self.OptionsString`))
  (if (`GameplayStatics.HasOption` _optionsstring "FarkleScore")
    (`self.SetTargetScore` (`KismetStringLibrary.Conv_StringToInt` (`GameplayStatics.ParseOption` _optionsstring "FarkleScore")))))

(event `RestartGame`
  (bind _firstplayer (`self.FirstPlayer`))
  (bind _secondplayer (`self.SecondPlayer`))
  (bind _asbp_farkle_player_controller (cast `/Game/Blueprints/Controllers/BP_FarklePlayerController` (`GameplayStatics.GetPlayerController` 0)))
  (`/Game/Blueprints/Controllers/BP_FarklePlayerController.RemoveWidget` _asbp_farkle_player_controller)
  (bind _asbp_farkle_player_controller_2 (cast `/Game/Blueprints/Controllers/BP_FarklePlayerController` (`GameplayStatics.GetPlayerController` 1)))
  (`/Game/Blueprints/Controllers/BP_FarklePlayerController.RemoveWidget` _asbp_farkle_player_controller_2)
  (set `BaseBoardPawn.TotalScore` 0 _firstplayer)
  (set `BaseBoardPawn.TurnScore` 0 _firstplayer)
  (set `BaseBoardPawn.SelectedScore` 0 _firstplayer)
  (set `BaseBoardPawn.TotalScore` 0 _secondplayer)
  (set `BaseBoardPawn.TurnScore` 0 _secondplayer)
  (set `BaseBoardPawn.SelectedScore` 0 _secondplayer)
  (`BaseBoardPawn.EndTurn` _secondplayer))

(event `self.EndGame`
  (params (winner :type "BaseBoardPawn Object Reference") (loser :type "BaseBoardPawn Object Reference"))
  (bind _returnvalue (`KismetStringLibrary.Contains` (`KismetSystemLibrary.GetDisplayName` winner) "FirstPlayer"))
  (bind _asbp_farkle_player_controller (cast `/Game/Blueprints/Controllers/BP_FarklePlayerController` (`GameplayStatics.GetPlayerController` 0)))
  (`/Game/Blueprints/Controllers/BP_FarklePlayerController.AddWidget` _asbp_farkle_player_controller _returnvalue)
  (bind _asbp_farkle_player_controller_2 (cast `/Game/Blueprints/Controllers/BP_FarklePlayerController` (`GameplayStatics.GetPlayerController` 1)))
  (`/Game/Blueprints/Controllers/BP_FarklePlayerController.AddWidget` _asbp_farkle_player_controller_2 (not _returnvalue)))

(event `self.K2_OnLogout`
  (params (ExitingController :type "Controller Object Reference"))
  (`GameplayStatics.OpenLevelBySoftObjectPtr` "/Game/Levels/MainMenuLevel.MainMenuLevel"))

(fn `UserConstructionScript`)