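; Player pawn for a Farkle dice board game, handling roll, pass and pause input plus turn-based camera movement.
; BeginPlay binds turn events, creates a hidden pause widget, and after a short delay adds the Farkle Enhanced Input mapping context.
; Turn end plays a timeline that blends the camera's relative location toward the track value, and turn start reverses it.
; Pause input toggles the widget and game pause together.
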(event `self.ReceiveBeginPlay`
  (`parent.ReceiveBeginPlay`)
  (add `self.OnEndTurn` (delegate `OnEndTurn_Event`))
  (add `self.OnStartTurn` (delegate `OnStartTurn_Event`))
  (bind _returnvalue (`|CreateWidget` "/Game/Blueprints/Widgets/WB_PauseMenu.WB_PauseMenu_C"))
  (bind _output_get (set `self.Pause Widget` _returnvalue))
  (`UserWidget.AddToViewport` _output_get 0)
  (`Widget.SetVisibility` _output_get "Hidden")
  (`KismetSystemLibrary.Delay` 1.0)
  (bind _asbp_farkle_player_controller (cast `/Game/Blueprints/Controllers/BP_FarklePlayerController` (`self.GetController`)))
  (`EnhancedInputSubsystemInterface.AddMappingContext` (pcsubsystem `EnhancedInputLocalPlayerSubsystem` _asbp_farkle_player_controller) "/Game/Input/FarkleInputMappingContext.FarkleInputMappingContext" 0 (struct)))

(event `OnEndTurn_Event`
  (bind _camera (`self.Camera`))
  (bind (_direction _newtrack_0) (`Timeline|Timeline` :!via `PlayFromStart` :!label _label)
    (:`Update`
      (`SceneComponent.K2_SetRelativeLocation` _camera (`KismetMathLibrary.VLerp` _newtrack_0 (`SceneComponent.RelativeLocation` _camera) 0.5) false false))))

(event `OnStartTurn_Event`
  (goto _label :!via `ReverseFromEnd`))

(event `EnhancedInput|/Game/Input/Actions/IA_Roll`
  (params (ActionValue :type Boolean) (ElapsedSeconds :type "Float (double-precision)") (TriggeredSeconds :type "Float (double-precision)") (InputAction :type "InputAction Object Reference" :default "/Game/Input/Actions/IA_Roll.IA_Roll"))
  (:`Started`
    (`self.RollDice`)))

(event `EnhancedInput|/Game/Input/Actions/IA_Pass`
  (params (ActionValue :type Boolean) (ElapsedSeconds :type "Float (double-precision)") (TriggeredSeconds :type "Float (double-precision)") (InputAction :type "InputAction Object Reference" :default "/Game/Input/Actions/IA_Pass.IA_Pass"))
  (:`Started`
    (`self.PassDice`)))

(event `EnhancedInput|/Game/Input/Actions/IA_Pause`
  (params (ActionValue :type Boolean) (ElapsedSeconds :type "Float (double-precision)") (TriggeredSeconds :type "Float (double-precision)") (InputAction :type "InputAction Object Reference" :default "/Game/Input/Actions/IA_Pause.IA_Pause"))
  (bind _pause_widget (`self.Pause Widget`))
  (:`Started`
    (switch `ESlateVisibility` (`Widget.GetVisibility` _pause_widget)
      (:`Visible`
        (`Widget.SetVisibility` _pause_widget "Hidden")
        (`GameplayStatics.SetGamePaused` false))
      (:`Hidden`
        (`Widget.SetVisibility` _pause_widget "Visible")
        (`GameplayStatics.SetGamePaused` true)))))

(fn `UserConstructionScript`)