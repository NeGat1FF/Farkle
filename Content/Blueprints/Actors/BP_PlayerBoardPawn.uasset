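; Player pawn for a Farkle dice game that takes Enhanced Input for rolling, passing and pausing.
; On BeginPlay it adds the Farkle input mapping, creates the pause menu widget and binds turn start and end events.
; Turn end plays a timeline that moves the camera by blending its current position halfway toward the track value each update; turn start reverses it.
; The pause input toggles both the menu and game pause.
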(event `self.ReceiveBeginPlay`
  (bind _returnvalue (`|CreateWidget` "/Game/Blueprints/Widgets/WB_PauseMenu.WB_PauseMenu_C"))
  (set `self.PauseWidget` _returnvalue)
  (`parent.ReceiveBeginPlay`)
  (bind _asplayer_controller (cast `PlayerController` (`self.GetController`)))
  (message `EnhancedInputSubsystemInterface.AddMappingContext` (pcsubsystem `EnhancedInputLocalPlayerSubsystem` _asplayer_controller) "/Game/Input/FarkleInputMappingContext.FarkleInputMappingContext" 0 (struct))
  (add `self.OnEndTurn` (delegate `OnEndTurn_Event`))
  (add `self.OnStartTurn` (delegate `OnStartTurn_Event`)))

(event `OnEndTurn_Event`
  (bind _camera (`self.Camera`))
  (bind (_direction _newtrack_0) (`Timeline|Timeline` :!via `PlayFromStart` :!label _label)
    (:`Update`
      (`SceneComponent.K2_SetRelativeLocation` _camera (`KismetMathLibrary.VLerp` _newtrack_0 (`SceneComponent.RelativeLocation` _camera) 0.5) false false))))

(event `OnStartTurn_Event`
  (goto _label :!via `ReverseFromEnd`))

(event `EnhancedInput|/Game/Input/Actions/IA_Roll`
  (params (ActionValue :type Boolean) (ElapsedSeconds :type "Float (double-precision)") (TriggeredSeconds :type "Float (double-precision)") (InputAction :type "InputAction Object Reference" :default "/Game/Input/Actions/IA_Roll.IA_Roll"))
  (:`Started`
    (`self.RollDice`)))

(event `EnhancedInput|/Game/Input/Actions/IA_Pass`
  (params (ActionValue :type Boolean) (ElapsedSeconds :type "Float (double-precision)") (TriggeredSeconds :type "Float (double-precision)") (InputAction :type "InputAction Object Reference" :default "/Game/Input/Actions/IA_Pass.IA_Pass"))
  (:`Started`
    (`self.PassDice`)))

(event `EnhancedInput|/Game/Input/Actions/IA_Pause`
  (params (ActionValue :type Boolean) (ElapsedSeconds :type "Float (double-precision)") (TriggeredSeconds :type "Float (double-precision)") (InputAction :type "InputAction Object Reference" :default "/Game/Input/Actions/IA_Pause.IA_Pause"))
  (bind _pausewidget (`self.PauseWidget`))
  (:`Started`
    (if (`Widget.IsInViewport` (`self.PauseWidget`))
      (`GameplayStatics.SetGamePaused` false)
      (`Widget.RemoveFromParent` _pausewidget)
      (else
        (`GameplayStatics.SetGamePaused` true)
        (`UserWidget.AddToViewport` _pausewidget 0)))))

(fn `UserConstructionScript`
  (`parent.UserConstructionScript`))