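; Player controller for the Farkle game that shows and clears the game-over screen.
; AddWidget creates a WB_GameOver widget owned by the controller, sets a translucent green or red tint and win or lose text from IsWinner, then adds it to the viewport.
; RemoveWidget clears the screen by removing all widgets, not just the game-over one.
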(event `AddWidget`
  (params (IsWinner :type Boolean))
  (bind _returnvalue (`|CreateWidget` "/Game/Blueprints/Widgets/WB_GameOver.WB_GameOver_C" self))
  (if IsWinner
    (bind _image_0 (`/Game/Blueprints/Widgets/WB_GameOver.Image_0` _returnvalue))
    (set `Image.ColorAndOpacity` (struct :`G` 1.0 :`A` 0.1) _image_0)
    (bind _textblock (`/Game/Blueprints/Widgets/WB_GameOver.TextBlock` _returnvalue))
    (set `TextBlock.Text` "YOU WON" _textblock)
    (else
      (set `Image.ColorAndOpacity` (struct :`R` 1.0 :`A` 0.1) _image_0)
      (set `TextBlock.Text` "YOU LOSE" _textblock)))
  (`UserWidget.AddToViewport` _returnvalue 0))

(event `RemoveWidget`
  (`WidgetLayoutLibrary.RemoveAllWidgets`))

(fn `UserConstructionScript`)