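; BP_FarkleGameState is the game state for a Farkle game that shows the end-of-game screen.
; On BeginPlay it binds its GameOver event to OnGameOver, which reports whether the human won.
; GameOver prints a debug string, creates a WB_GameOver widget with a win or lose message and matching tint, and adds it to the viewport.
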(event `self.ReceiveBeginPlay`
  (add `self.OnGameOver` (delegate `GameOver`)))

(event `GameOver` :!signature `self.OnGameOver`
  (params (bIsHumanWinner :type Boolean))
  (`KismetSystemLibrary.PrintText` "Hello")
  (bind _returnvalue (`|CreateWidget` "/Game/Blueprints/WB_GameOver.WB_GameOver_C"))
  (if bIsHumanWinner
    (bind _textblock (`/Game/Blueprints/WB_GameOver.TextBlock` _returnvalue))
    (set `TextBlock.Text` "YOU WON" _textblock)
    (bind _image_0 (`/Game/Blueprints/WB_GameOver.Image_0` _returnvalue))
    (`Image.SetColorAndOpacity` _image_0 (struct :`G` 1.0 :`A` 0.5))
    (else
      (set `TextBlock.Text` "YOU LOSE" _textblock)
      (`Image.SetColorAndOpacity` _image_0 (struct :`A` 0.5))))
  (`UserWidget.AddToViewport` _returnvalue 0))

(fn `UserConstructionScript`)